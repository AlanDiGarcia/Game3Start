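; BP_PatrolRoute is a patrol route that supplies world-space waypoints from the points of a spline.
; GetPatrolPointLocation calls IncrementPatrolPoint, then returns the spline point at the new index, so every query advances the route.
; The index steps by Direction and resets to zero on reaching the point count, with no lower-bound check.
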(event Custom|Increment%20Patrol%20Point
  (Variables|Default|SetPatrol%20Index (+ (Variables|Default|GetPatrol%20Index) (Variables|Default|GetDirection)))
  (if (not (< (Variables|Default|GetPatrol%20Index) (Spline|GetNumberOfSplinePoints (Variables|Default|GetSpline))))
    (Variables|Default|SetPatrol%20Index 0)))

(fn ConstructionScript)

(fn GetPatrolPointLocation
  (CallFunction|IncrementPatrolPoint)
  (return (Spline|GetLocationatSplinePoint (Variables|Default|GetSpline) (Variables|Default|GetPatrol%20Index) "World")))