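; BP_CameraDoor is a door that briefly takes over the player's view while it opens.
; ActivateDoor registers the door in GM_SaveState's LevelSave, blends the view to itself, opens, then after a pause blends to the supplied view target at twice the speed.
; OpenDoor plays a Timeline that lerps the Door component downward.
; Saving stores only the actor reference, added uniquely to DoorRef.
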(event Custom|Activate%20Door
  (params (NewViewTarget :type Actor%20Object%20Reference))
  (CallFunction|SaveDoorState)
  (Game|Player|SetViewTargetwithBlend (Game|GetPlayerController 0) self (Variables|Default|GetBlend%20Time) "VTBlend_Cubic" 0.0 true)
  (Utilities|FlowControl|Delay (Variables|Default|GetBlend%20Time))
  (CallFunction|OpenDoor)
  (Utilities|FlowControl|Delay 3.0)
  (Game|Player|SetViewTargetwithBlend (Game|GetPlayerController 0) NewViewTarget (/ (Variables|Default|GetBlend%20Time) 2.0) "VTBlend_Cubic" 0.0 false))

(event Custom|Open%20Door
  (bind _newtrack_0 (Timeline|Timeline Play)
    (:Update
      (Transformation|SetRelativeLocation (Variables|Default|GetDoor) (Math|Vector|Lerp(Vector) "0.000000,0.000000,150.000000" "0.000000,0.000000,-130.000000" _newtrack_0) false false))))

(event Custom|Save%20Door%20State
  (bind _asgm_save_state (Utilities|Casting|CastToGM_SaveState (Game|GetGameMode)))
  (Utilities|Array|AddUnique (Variables|/Game/NewSaves/SG_LevelState.SG_LevelState_C|GetDoor%20Ref (Variables|/Game/NewSaves/GM_SaveState.GM_SaveState_C|GetLevel%20Save _asgm_save_state)) self))

(fn ConstructionScript)