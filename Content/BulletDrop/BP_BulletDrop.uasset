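; Bullet drop test actor that steps a simulated projectile along a gravity arc using line traces, alongside Unreal's built-in path prediction.
; A looping timer adds constant world-X travel and accumulating gravity each step, drawing a debug trace per segment.
; On a hit it resets to the Arrow's starting position, then recomputes the step values and redraws the predicted path.
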(event Custom|Predict%20Bullet%20Drop
  (Variables|Default|SetOld%20Location (Variables|Default|GetLocation))
  (Variables|Default|SetAdditive%20Gravity (+ (Variables|Default|GetAdditive%20Gravity) (Variables|Default|GetGravity%20per%20Section)))
  (Variables|Default|SetLocation (+ (Variables|Default|GetLocation) (Math|Vector|MakeVector (Variables|Default|GetLaunch%20Velocity) 0.0 (Variables|Default|GetAdditive%20Gravity))))
  (bind _returnvalue (Collision|LineTraceByChannel (Variables|Default|GetOld%20Location) (Variables|Default|GetLocation) "TraceTypeQuery2" false 0 "ForDuration" true "(R=1.000000,G=0.000000,B=0.000000,A=1.000000)" "(R=0.000000,G=1.000000,B=0.000000,A=1.000000)" 0.5))
  (if _returnvalue
    (Variables|Default|SetLocation (Variables|Default|GetStart%20Location))
    (Variables|Default|SetAdditive%20Gravity 0.0)
    (CallFunction|UpdateProjectilePath)))

(event Custom|Update%20Projectile%20Path
  (Variables|Default|SetLaunch%20Velocity (* (.x (Variables|Default|GetStart%20Velocity)) (Variables|Default|GetTime)))
  (Variables|Default|SetGravity%20per%20Section (* (Variables|Default|GetGravity) (Math|Float|Square (Variables|Default|GetTime))))
  (Class|GameplayStatics|BlueprintPredictProjectilePathAdvanced (Utilities|Struct|MakePredictProjectilePathParams (Transformation|GetWorldLocation (Variables|Default|GetArrow)) (Variables|Default|GetStart%20Velocity) true 3.0 1.0 true "ECC_WorldStatic" "ObjectTypeQuery1" 0 2e+01 -9.8e+02 "ForDuration" 1.0 false)))

(event EventBeginPlay
  (CallFunction|UpdateProjectilePath)
  (Variables|Default|SetStart%20Location (Transformation|GetWorldLocation (Variables|Default|GetArrow)))
  (Utilities|Time|SetTimerbyEvent (delegate Custom|Predict%20Bullet%20Drop) (Variables|Default|GetTime) true))

(fn ConstructionScript)