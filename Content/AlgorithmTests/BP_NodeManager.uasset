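; BP_NodeManager is an algorithm-test actor that scatters BP_Node actors and visualizes the path through them in spawn order.
; A looping timer spawns a node at a random point in a box around the manager and records it in an array.
; EndSpawning pauses the timer, caches node locations and calls DrawLines, which links consecutive nodes with debug lines in an HSV-interpolated color gradient.
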(event Custom|Spawn%20Node
  (bind _returnvalue (Game|SpawnActorfromClass "/Game/AlgorithmTests/BP_Node.BP_Node_C" (Math|Transform|MakeTransform (Math|Random|RandomPointinBoundingBox (Transformation|GetActorLocation) "750.000000,750.000000,400.000000") "0, 0, 0" "1.000000,1.000000,1.000000") "Undefined" "MultiplyWithRoot" 0 0))
  (Utilities|Array|AddUnique (Variables|Default|GetBP%20Node%20Array) _returnvalue))

(event Custom|End%20Spawning
  (Development|PrintString "Stop Spawning" true true "(R=1.000000,G=0.552337,B=0.000000,A=1.000000)" 5.0)
  (Utilities|Time|PauseTimerbyHandle (Variables|Default|GetSpawing%20Timer))
  (for _array_element (Variables|Default|GetBP%20Node%20Array)
    (Utilities|Array|AddUnique (Variables|Default|GetBP%20Node%20Location) (Transformation|GetActorLocation _array_element)))
  (CallFunction|DrawLines))

(event Custom|Draw%20Lines
  (Development|PrintString "Draw Lines" true true "(R=0.756166,G=1.000000,B=0.000000,A=1.000000)" 5.0)
  (for _index (range 0 (Utilities|Array|Length (Variables|Default|GetBP%20Node%20Array)))
    (Variables|Default|SetNode%20Index (+ _index 1))
    (if (not (Math|Vector|VectorIsZero (Utilities|Array|Get(acopy) (Variables|Default|GetBP%20Node%20Location) (Variables|Default|GetNode%20Index))))
      (Rendering|Debug|DrawDebugLine (Utilities|Array|Get(acopy) (Variables|Default|GetBP%20Node%20Location) _index) (Utilities|Array|Get(acopy) (Variables|Default|GetBP%20Node%20Location) (Variables|Default|GetNode%20Index)) (Class|KismetMathLibrary|LinearColorLerpUsingHSV "(R=1.000000,G=0.063817,B=0.000000,A=1.000000)" "(R=0.000000,G=1.000000,B=0.797719,A=1.000000)" (/ (Math|Conversions|ToFloat(Integer) _index) 1e+01)) 1e+02 5.0))))

(event EventBeginPlay
  (bind _returnvalue (Utilities|Time|SetTimerbyEvent (delegate Custom|Spawn%20Node) 0.5 true))
  (Variables|Default|SetSpawing%20Timer _returnvalue))

(fn ConstructionScript)