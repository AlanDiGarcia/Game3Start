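; Test actor that visualizes HSV color interpolation with debug spheres.
; On BeginPlay a loop draws a temporary vertical column of spheres rising from the actor's location, with an accumulating Step value driving both height and the HSV lerp from red to turquoise-green.
; A disconnected Timeline variant, which would animate a red-to-yellow lerp at the actor's location, never runs.
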(event EventBeginPlay
  (bind _returnvalue (Transformation|GetActorLocation))
  (for _index (range 0 9)
    (Rendering|Debug|DrawDebugSphere (Math|Vector|MakeVector (.x _returnvalue) (.y _returnvalue) (+ (* (Variables|Default|GetStep) 1e+03) (.z _returnvalue))) 1e+02 12 (Class|KismetMathLibrary|LinearColorLerpUsingHSV "(R=1.000000,G=0.004207,B=0.000000,A=1.000000)" "(R=0.000000,G=1.000000,B=0.762499,A=1.000000)" (Variables|Default|GetStep)) 1e+01 5.0)
    (Variables|Default|SetStep (+ (Variables|Default|GetStep) 0.1))))

(fn ConstructionScript)