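; GM_BallMainMenu is the main menu game mode for the Ball game, which trims local multiplayer down to the primary player.
; On BeginPlay, if more than one local player controller exists, it loops over controller IDs 1 to 3 and removes those players without destroying their pawns.
; The only other logic is disconnected debug prints of the local player count.
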(event EventBeginPlay
  ;[0.05098 0.05098 0.05098 1 30] Player Connection / Disconnection
  (if (> (Class|GameplayStatics|GetNumLocalPlayerControllers) 1)
    (for _index (range 1 3)
      (Class|GameplayStatics|RemovePlayer (Class|GameplayStatics|GetPlayerControllerfromID _index) false))))

(fn ConstructionScript)