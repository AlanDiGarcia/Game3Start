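; Game mode for the ball game that tracks connected player controllers and creates local players on BeginPlay.
; Login and controller-swap events add controllers to AllPlayerControllers, and logout removes them.
; SpawnPlayer, not called within this Blueprint, destroys any existing pawn, then spawns and possesses a BP_BallCharacter at the PlayerStart indexed by the controller count.
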(event EventBeginPlay
  (Spawn|LocalPlayer (Variables|Default|GetLocal%20Players)))

(event EventPostLogin
  (params (NewPlayer :type Player%20Controller%20Object%20Reference))
  ;[0.05098 0.05098 0.05098 1 30] Player Connection / Disconnection
  ;;[0.05098 0.05098 0.05098 1 30] Players Log In
  (bind _returnvalue (Utilities|Array|Add (Variables|Default|GetAll%20Player%20Controllers) NewPlayer))
  (Development|PrintString (Utilities|String|Append "Player: " (Utilities|String|ToString(Integer) _returnvalue) " Joined") true true "(R=0.255044,G=0.000000,B=1.000000,A=1.000000)"))

(event EventOnSwapPlayerControllers
  (params (OldPC :type Player%20Controller%20Object%20Reference) (NewPC :type Player%20Controller%20Object%20Reference))
  ;[0.05098 0.05098 0.05098 1 30] Player Connection / Disconnection
  ;;[0.05098 0.05098 0.05098 1 30] Players Switch Level
  (Utilities|Array|Add (Variables|Default|GetAll%20Player%20Controllers) NewPC))

(event EventOnLogout
  (params (ExitingController :type Controller%20Object%20Reference))
  ;[0.05098 0.05098 0.05098 1 30] Player Connection / Disconnection
  ;;[0.05098 0.05098 0.05098 1 30] Players Log Out
  (bind _aspc_ball_player_controller (Utilities|Casting|CastToPC_BallPlayerController ExitingController))
  (Utilities|Array|RemoveItem (Variables|Default|GetAll%20Player%20Controllers) _aspc_ball_player_controller))

(fn ConstructionScript)

(fn FindPlayerStarts
  (params (Player%20Slots :type Integer))
  (bind _outactors (Actor|GetAllActorsOfClass "/Script/Engine.PlayerStart"))
  (return (Transformation|GetActorTransform (Utilities|Array|Get(acopy) _outactors Player%20Slots))))

(fn SpawnPlayer
  (params (Player%20Controller :type Player%20Controller%20Object%20Reference))
  (bind _returnvalue (Pawn|GetControlledPawn Player%20Controller))
  (Utilities|IsValid _returnvalue
    (:Is%20Valid
      (Actor|DestroyActor _returnvalue))
    (:Is%20Not%20Valid
      (Development|PrintString "No Pawn" true true "(R=1.000000,G=0.000000,B=0.034709,A=1.000000)" 7.0)))
  (bind _returnvalue_2 (Game|SpawnActorfromClass "/Game/Ball/BP_BallCharacter.BP_BallCharacter_C" (Spawn|FindPlayerStarts (Utilities|Array|Length (Variables|Default|GetAll%20Player%20Controllers))) "Undefined" "MultiplyWithRoot" 0 0))
  (Pawn|Possess Player%20Controller _returnvalue_2))

(fn LocalPlayer
  (params (Local%20Players :type Integer))
  (Utilities|FlowControl|ForLoopwithBreak 1 Local%20Players
    (:LoopBody
      (Class|GameplayStatics|CreatePlayer -1))))