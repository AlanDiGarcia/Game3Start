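; Player controller for the ball game that requests a player spawn from the game mode when play begins.
; On BeginPlay, the local controller calls SRSpawnPlayer, grouped under server actions, which casts to GM_BallGameMode and passes itself to SpawnPlayer.
; AddPlayerController is an empty event, and the logic that would assign the controller to BP_BallCharacter is disconnected.
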(event Custom|SR%20Spawn%20Player
  ;[0.05098 0.05098 0.05098 1 30] Actions to Server
  (bind _asgm_ball_game_mode (Utilities|Casting|CastToGM_BallGameMode (Game|GetGameMode)))
  (Default|SpawnPlayer _asgm_ball_game_mode self))

(event Custom|Add%20Player%20Controller)

(event EventBeginPlay
  ;[0.05098 0.05098 0.05098 1 30] Actions to Server
  (if (Pawn|IsLocalPlayerController)
    (CallFunction|SRSpawnPlayer)))

(fn ConstructionScript)