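; BP_PowerBox is a pickup box that powers up an overlapping ball character that is not already powered.
; A Spin timeline, started at a random time, rotates the cube while a looping timer swaps in random materials from an array.
; On pickup it hides and ignores collision, then reappears after HideDuration with overlap responses restored.
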(event OnComponentBeginOverlap(Box)
  (params (OverlappedComponent :type Primitive%20Component%20Object%20Reference) (OtherActor :type Actor%20Object%20Reference) (OtherComp :type Primitive%20Component%20Object%20Reference) (OtherBodyIndex :type Integer) (bFromSweep :type Boolean) (SweepResult :type Hit%20Result%20Structure%20%28by%20ref%29))
  (switch string (Utilities|GetClassDisplayName (Utilities|GetClass OtherActor))
    (:BP_BallCharacter_C
      (bind _asbp_ball_character (Utilities|Casting|CastToBP_BallCharacter OtherActor))
      (if (not (Variables|/Game/Ball/BP_BallCharacter.BP_BallCharacter_C|GetPowered _asbp_ball_character))
        (Default|PowerUp _asbp_ball_character)
        (CallFunction|Hide)
        (Development|PrintString "Touched" true true "(R=1.000000,G=0.000000,B=0.147743,A=1.000000)")))))

(event Custom|Change%20Color
  (bind _materials (Variables|Default|GetMaterials))
  (Rendering|Material|SetMaterial (Variables|Default|GetCube) 0 (Utilities|Array|Get(acopy) _materials (Math|Random|RandomIntegerinRange 0 (- (Utilities|Array|Length _materials) 1)))))

(event Custom|Hide
  (Rendering|SetActorHiddenInGame true)
  (Collision|SetCollisionResponsetoAllChannels (Variables|Default|GetBox) "ECR_Ignore")
  (Utilities|FlowControl|RetriggerableDelay (Variables|Default|GetHide%20Duration))
  (CallFunction|Return))

(event Custom|Return
  (Rendering|SetActorHiddenInGame false)
  (Collision|SetCollisionResponsetoAllChannels (Variables|Default|GetBox) "ECR_Overlap"))

(event EventBeginPlay
  (Utilities|Time|SetTimerbyEvent (delegate Custom|Change%20Color) 0.4 true)
  (Utilities|FlowControl|Sequence
    (:then_0
      (bind _newtrack_0 (Timeline|Spin SetNewTime)
        (:Update
          (Transformation|SetWorldRotation (Variables|Default|GetCube) (Math|Rotator|Lerp(Rotator) "0, 0, 0" "0.000000,360.000000,0.000000" _newtrack_0) false false))))
    (:then_1
      (Timeline|Spin Play))))

(fn ConstructionScript)