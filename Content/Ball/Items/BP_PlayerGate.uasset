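; BP_PlayerGate is a gate that opens once two buttons are active at the same time.
; ActivateDoor records each button's state by index in a bool array, then TestDoor checks that the first two entries are both true.
; When they are, OpenDoor plays a Timeline that lerps the Cube's relative location upward.
; The file has no logic to close the gate again.
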(event Custom|Open%20Door
  (bind _newtrack_0 (Timeline|Timeline Play)
    (:Update
      (Transformation|SetRelativeLocation (Variables|Default|GetCube) (Math|Vector|Lerp(Vector) "0, 0, 0" "0.000000,0.000000,500.000000" _newtrack_0) false false))))

(event Custom|Activate%20Door
  (params (Button%20Number :type Integer) (Button%20Bool :type Boolean))
  (Utilities|Array|SetArrayElem (Variables|Default|GetButton%20Bool%20Array) Button%20Number Button%20Bool true)
  (CallFunction|TestDoor))

(event Custom|Test%20Door
  (bind _button_bool_array (Variables|Default|GetButton%20Bool%20Array))
  (if (> (Utilities|Array|Length _button_bool_array) 1)
    (if (and (Utilities|Array|Get(acopy) _button_bool_array 1) (Utilities|Array|Get(acopy) _button_bool_array))
      (CallFunction|OpenDoor))))

(fn ConstructionScript)