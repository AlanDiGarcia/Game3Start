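; Spinning coin pickup that temporarily disappears when a BP_BallCharacter overlaps it.
; A timeline spins the mesh from a random start time so each coin's rotation is offset.
; On authority, overlap plays the pickup sound and flips Hiding, then flips it back after a retriggerable delay.
; OnRep_Hiding toggles visibility and Box collision, counterintuitively calling Return when Hiding is true and Hide when false.
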(event OnComponentBeginOverlap(StaticMesh)
  (params (OverlappedComponent :type Primitive%20Component%20Object%20Reference) (OtherActor :type Actor%20Object%20Reference) (OtherComp :type Primitive%20Component%20Object%20Reference) (OtherBodyIndex :type Integer) (bFromSweep :type Boolean) (SweepResult :type Hit%20Result%20Structure%20%28by%20ref%29))
  (switch string (Utilities|GetClassDisplayName (Utilities|GetClass OtherActor))
    (:BP_BallCharacter_C
      (Networking|SwitchHasAuthority
        (:Authority
          (CallFunction|ToggleCoin)
          (Audio|PlaySoundatLocation "/Game/Audio/SFX/Pickup_Coin.Pickup_Coin" (Transformation|GetWorldLocation (Variables|Default|GetStaticMesh)) "0, 0, 0" 1.0 1.0 0.0 "/Game/Ball/Sound/ATT_Boost.ATT_Boost" 0 0 0))))))

(event Custom|Hide
  (Rendering|SetActorHiddenInGame true)
  (Collision|SetCollisionResponsetoAllChannels (Variables|Default|GetBox) "ECR_Ignore"))

(event Custom|Return
  (Rendering|SetActorHiddenInGame false)
  (Collision|SetCollisionResponsetoAllChannels (Variables|Default|GetBox) "ECR_Overlap"))

(event Custom|Toggle%20Coin
  (Variables|Default|SetHiding (not (Variables|Default|GetHiding)))
  (Utilities|FlowControl|RetriggerableDelay (Variables|Default|GetHide%20Duration))
  (Variables|Default|SetHiding (not (Variables|Default|GetHiding))))

(event EventBeginPlay
  (Utilities|FlowControl|Sequence
    (:then_0
      (bind _newtrack_0 (Timeline|Timeline SetNewTime)
        (:Update
          (Transformation|SetWorldRotation (Variables|Default|GetStaticMesh) (Math|Rotator|Lerp(Rotator) "0, 0, 0" "0.000000,360.000000,0.000000" _newtrack_0) false false))))
    (:then_1
      (Timeline|Timeline Play))))

(fn ConstructionScript)

(fn OnRepHiding
  (if (Variables|Default|GetHiding)
    (CallFunction|Return)
    (else
      (CallFunction|Hide))))