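; BP_PlayerGateButton is a pressure-style button that reports to a player gate when a ball character enters or leaves its trigger box.
; Overlap begin and end set ButtonBool true or false, then call ActivateDoor on BP_PlayerGate with the button's number and state.
; The ball is identified by a switch on class display name, and GetActorOfClass fetches a single gate rather than using an assigned reference.
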(event OnComponentBeginOverlap(Box)
  (params (OverlappedComponent :type Primitive%20Component%20Object%20Reference) (OtherActor :type Actor%20Object%20Reference) (OtherComp :type Primitive%20Component%20Object%20Reference) (OtherBodyIndex :type Integer) (bFromSweep :type Boolean) (SweepResult :type Hit%20Result%20Structure%20%28by%20ref%29))
  (switch string (Utilities|GetClassDisplayName (Utilities|GetClass OtherActor))
    (:BP_BallCharacter_C
      (Variables|Default|SetButton%20Bool true)
      (bind _returnvalue (Actor|GetActorOfClass "/Game/Ball/Items/BP_PlayerGate.BP_PlayerGate_C"))
      (Default|ActivateDoor _returnvalue (Variables|Default|GetButton%20Number) (Variables|Default|GetButton%20Bool)))))

(event OnComponentEndOverlap(Box)
  (params (OverlappedComponent :type Primitive%20Component%20Object%20Reference) (OtherActor :type Actor%20Object%20Reference) (OtherComp :type Primitive%20Component%20Object%20Reference) (OtherBodyIndex :type Integer))
  (switch string (Utilities|GetClassDisplayName (Utilities|GetClass OtherActor))
    (:BP_BallCharacter_C
      (Variables|Default|SetButton%20Bool false)
      (bind _returnvalue (Actor|GetActorOfClass "/Game/Ball/Items/BP_PlayerGate.BP_PlayerGate_C"))
      (Default|ActivateDoor _returnvalue (Variables|Default|GetButton%20Number) (Variables|Default|GetButton%20Bool)))))

(fn ConstructionScript)