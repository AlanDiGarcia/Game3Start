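; BP_SpawnPoint is a checkpoint for the ball game that updates the player's respawn location on contact.
; When something overlaps its Box, it switches on the class display name and casts matches to BP_BallCharacter.
; It then passes a point just above its Cube to the character's SetSpawnpoint and plays a coin pickup sound at the ball.
; Nothing disables the trigger, so every new overlap repeats this.
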(event OnComponentBeginOverlap(Box)
  (params (OverlappedComponent :type Primitive%20Component%20Object%20Reference) (OtherActor :type Actor%20Object%20Reference) (OtherComp :type Primitive%20Component%20Object%20Reference) (OtherBodyIndex :type Integer) (bFromSweep :type Boolean) (SweepResult :type Hit%20Result%20Structure%20%28by%20ref%29))
  (bind _cube (Variables|Default|GetCube))
  (bind _returnvalue (Transformation|GetWorldLocation _cube))
  (switch string (Utilities|GetClassDisplayName (Utilities|GetClass OtherActor))
    (:BP_BallCharacter_C
      (bind _asbp_ball_character (Utilities|Casting|CastToBP_BallCharacter OtherActor))
      (Default|SetSpawnpoint _asbp_ball_character (Math|Vector|MakeVector (.x _returnvalue) (.y _returnvalue) (+ (.z _returnvalue) 1e+02)))
      (Audio|PlaySoundatLocation "/Game/Audio/SFX/Pickup_Coin2.Pickup_Coin2" (Transformation|GetWorldLocation (Variables|/Game/Ball/BP_BallCharacter.BP_BallCharacter_C|GetSphere _asbp_ball_character)) "0, 0, 0" 1.0 1.0 0.0 "/Game/Ball/Sound/ATT_Boost.ATT_Boost" 0 0 0))))

(fn ConstructionScript)