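; Game mode that manages per-level save state, using the current level name as the save slot.
; On BeginPlay it loads or creates an SG_LevelState, has it restore collected coins, door state and slow motion, and moves the player to the saved transform.
; Checkpoint stores the player transform and saves.
; FinishedLevel zeroes that transform before saving; a zero location skips repositioning on load.
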(event Custom|Save%20Game
  (bind _returnvalue (Game|GetCurrentLevelName true))
  (bind _returnvalue_2 (SaveGame|SaveGametoSlot (Variables|Default|GetLevel%20Save) _returnvalue))
  (if _returnvalue_2
    (Development|PrintString "Saved" true true "(R=0.008017,G=1.000000,B=0.000000,A=1.000000)" 3.0)))

(event Custom|Load%20Game
  (bind _returnvalue (Game|GetCurrentLevelName true))
  (bind _output_get (Variables|Default|SetSlot%20Name _returnvalue))
  (bind _returnvalue_2 (SaveGame|DoesSaveGameExist _output_get))
  (if _returnvalue_2
    (bind _returnvalue_3 (SaveGame|LoadGamefromSlot (Variables|Default|GetSlot%20Name)))
    (bind _assg_level_state (Utilities|Casting|CastToSG_LevelState _returnvalue_3))
    (Variables|Default|SetLevel%20Save _assg_level_state)
    (Default|LoadCollectedCoins (Variables|Default|GetLevel%20Save))
    (Default|LoadDoorState (Variables|Default|GetLevel%20Save))
    (Default|LoadSlowmotion (Variables|Default|GetLevel%20Save))
    (if (not (Class|KismetMathLibrary|EqualExactlyVectorVector (.location (Variables|/Game/NewSaves/SG_LevelState.SG_LevelState_C|GetPlayer%20Transform (Variables|Default|GetLevel%20Save))) "0, 0, 0"))
      (Transformation|SetWorldTransform (Variables|/Script/Engine.Character|GetCapsuleComponent (Game|GetPlayerCharacter 0)) (Variables|/Game/NewSaves/SG_LevelState.SG_LevelState_C|GetPlayer%20Transform (Variables|Default|GetLevel%20Save)) false false))
    (else
      (bind _returnvalue_4 (SaveGame|CreateSaveGameObject "/Game/NewSaves/SG_LevelState.SG_LevelState_C"))
      (Variables|Default|SetLevel%20Save _returnvalue_4))))

(event EventBeginPlay
  (CallFunction|LoadGame))

(fn ConstructionScript)

(fn Checkpoint
  (params (Player%20Transform :type Transform))
  (Variables|/Game/NewSaves/SG_LevelState.SG_LevelState_C|SetPlayer%20Transform (Variables|Default|GetLevel%20Save) Player%20Transform)
  (CallFunction|SaveGame))

(fn FinishedLevel
  (Variables|/Game/NewSaves/SG_LevelState.SG_LevelState_C|SetPlayer%20Transform (Variables|Default|GetLevel%20Save) (Math|Transform|MakeTransform "0, 0, 0" "0, 0, 0" "1.000000,1.000000,1.000000"))
  (CallFunction|SaveGame))