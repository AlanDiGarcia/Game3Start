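; BP_Weapon is a weapon display actor that shows a weapon's mesh and stats from a passed-in weapon struct.
; SetText fills text components with weapon type, damage type and a randomized range around base damage, colors the damage type by element, and starts a short lifespan.
; SetMesh applies the struct's mesh and scale, then picks an overlay material for Fire, Ice, Lightning or Poison.
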(event Custom|Set%20Mesh
  (params (S%20Weapon :type S%20Weapon%20Structure))
  (bind _weapon_body (Variables|Default|GetWeapon%20Body))
  (Components|StaticMesh|SetStaticMesh (Variables|Default|GetWeapon%20Body) (.weaponmesh S%20Weapon))
  (Transformation|SetWorldScale3D (Variables|Default|GetWeapon%20Body) (.weaponscale S%20Weapon))
  (switch Utilities|FlowControl|Switch|SwitchonE_DamageType (.damagetype S%20Weapon)
    (:NewEnumerator2
      (Rendering|Material|SetOverlayMaterial _weapon_body "/Engine/VREditor/BasicMeshes/MI_Cube_03.MI_Cube_03" :!class /Script/Engine.MeshComponent))
    (:NewEnumerator3
      (Rendering|Material|SetOverlayMaterial _weapon_body "/Engine/VREditor/BasicMeshes/MI_Cube_02.MI_Cube_02" :!class /Script/Engine.MeshComponent))
    (:NewEnumerator5
      (Rendering|Material|SetOverlayMaterial _weapon_body "/Engine/VREditor/BasicMeshes/MI_Cube_01.MI_Cube_01" :!class /Script/Engine.MeshComponent))
    (:NewEnumerator6
      (Rendering|Material|SetOverlayMaterial _weapon_body "/Engine/VREditor/BasicMeshes/MI_Pyramid_01.MI_Pyramid_01" :!class /Script/Engine.MeshComponent))))

(event Custom|Set%20Text
  (params (S_Weapon :type S%20Weapon%20Structure))
  (bind _damagetypetext (Variables|Default|GetDamageTypeText))
  (Actor|SetLifeSpan 5.0)
  (Rendering|Components|TextRender|SetText (Variables|Default|GetWeaponTypeText) (Utilities|Text|ToText(String) (Utilities|String|EnumtoString (.weapontype S_Weapon))))
  (Rendering|Components|TextRender|SetText (Variables|Default|GetDamageTypeText) (Utilities|Text|ToText(String) (Utilities|String|EnumtoString (.damagetype S_Weapon))))
  (Rendering|Components|TextRender|SetText (Variables|Default|GetDamageText) (Utilities|Text|ToText(String) (Utilities|String|Append (Utilities|String|ToString(Integer) (- (.basedamage S_Weapon) (Math|Random|RandomIntegerinRange 0 3))) "-" (Utilities|String|ToString(Integer) (+ (.basedamage S_Weapon) (Math|Random|RandomIntegerinRange 1 3))))))
  (switch Utilities|FlowControl|Switch|SwitchonE_DamageType (.damagetype S_Weapon)
    (:NewEnumerator2
      (Rendering|Components|TextRender|SetTextRenderColor _damagetypetext (Math|Color|MakeColor 0 10 90 0)))
    (:NewEnumerator3
      (Rendering|Components|TextRender|SetTextRenderColor _damagetypetext (Math|Color|MakeColor 90 40 0 0)))
    (:NewEnumerator5
      (Rendering|Components|TextRender|SetTextRenderColor _damagetypetext (Math|Color|MakeColor 0 70 70 0)))
    (:NewEnumerator6
      (Rendering|Components|TextRender|SetTextRenderColor _damagetypetext (Math|Color|MakeColor 90 10 90 0)))))

(fn ConstructionScript)