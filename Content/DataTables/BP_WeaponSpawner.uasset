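; Weapon spawner that spawns a random weapon when the third-person character overlaps its sphere.
; The overlap identifies the character by class display name, then picks a random row from the DT_Weapons data table.
; It spawns a BP_Weapon at the cylinder's X/Y and a fixed height, then passes the row to set its text and mesh.
; Every qualifying overlap spawns another weapon, and a missing row prints a debug message.
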(event OnComponentBeginOverlap(Sphere)
  (params (OverlappedComponent :type Primitive%20Component%20Object%20Reference) (OtherActor :type Actor%20Object%20Reference) (OtherComp :type Primitive%20Component%20Object%20Reference) (OtherBodyIndex :type Integer) (bFromSweep :type Boolean) (SweepResult :type Hit%20Result%20Structure%20%28by%20ref%29))
  (switch string (Utilities|GetClassDisplayName (Utilities|GetClass OtherActor))
    (:BP_ThirdPersonCharacter_C
      (CallFunction|SpawnWeapon))))

(event Custom|Spawn%20Weapon
  (bind _cylinder (Variables|Default|GetCylinder))
  (bind _returnvalue (Transformation|GetWorldLocation _cylinder))
  (bind _outrownames (DataTable|GetDataTableRowNames "/Game/DataTables/DT_Weapons.DT_Weapons"))
  (bind _returnvalue_2 (Utilities|GetDataTableRow "/Game/DataTables/DT_Weapons.DT_Weapons" (.OutItem (Utilities|Array|Random _outrownames)))
    (:then
      (Variables|Default|SetS%20Weapon _returnvalue_2)
      (bind _returnvalue_3 (Game|SpawnActorfromClass "/Game/DataTables/BP_Weapon.BP_Weapon_C" (Math|Transform|MakeTransform (Math|Vector|MakeVector (.x _returnvalue) (.y _returnvalue) 1e+02) "0, 0, 0" "1.000000,1.000000,1.000000") "Undefined" "MultiplyWithRoot" 0 0))
      (Default|SetText _returnvalue_3 (Variables|Default|GetS%20Weapon))
      (Default|SetMesh _returnvalue_3 (Variables|Default|GetS%20Weapon)))
    (:RowNotFound
      (Development|PrintString "Row Not Found" true true "(R=1.000000,G=0.252350,B=0.000000,A=1.000000)" 4.0))))

(fn ConstructionScript)