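; Dialogue trigger actor that shows a press-E prompt and enables conversation while the third-person character overlaps its box.
; Each ActivateDialogue call reads the next DT_Dialogue row by index, updating the widget's text, speaker portrait and emotion image via enum-to-material switches.
; A DoOnce guards adding the dialogue widget to the viewport.
; After the last row, it removes the widget, resets the index and DoOnce, and disables dialogue.
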(event OnComponentBeginOverlap(Box)
  (params (OverlappedComponent :type Primitive%20Component%20Object%20Reference) (OtherActor :type Actor%20Object%20Reference) (OtherComp :type Primitive%20Component%20Object%20Reference) (OtherBodyIndex :type Integer) (bFromSweep :type Boolean) (SweepResult :type Hit%20Result%20Structure%20%28by%20ref%29))
  (switch string (Utilities|GetClassDisplayName (Utilities|GetClass OtherActor))
    (:BP_ThirdPersonCharacter_C
      (UserInterface|Viewport|AddtoViewport (Variables|Default|GetWB%20PressE%20Ref) 0)
      (Variables|Default|SetDialogue true))))

(event OnComponentEndOverlap(Box)
  (params (OverlappedComponent :type Primitive%20Component%20Object%20Reference) (OtherActor :type Actor%20Object%20Reference) (OtherComp :type Primitive%20Component%20Object%20Reference) (OtherBodyIndex :type Integer))
  (switch string (Utilities|GetClassDisplayName (Utilities|GetClass OtherActor))
    (:BP_ThirdPersonCharacter_C
      (Widget|RemovefromParent (Variables|Default|GetWB%20PressE%20Ref))
      (Variables|Default|SetDialogue false))))

(event Custom|Set%20Emotion
  (params (E%20Emotion :type E_Emotion%20Enum :default "NewEnumerator0"))
  (bind _wb_dialogue_ref (Variables|Default|GetWB%20Dialogue%20Ref))
  (bind _image_emotion (Variables|/Game/DataTables/Dialogue/WB_Dialogue.WB_Dialogue_C|GetImage_Emotion _wb_dialogue_ref))
  (switch Utilities|FlowControl|Switch|SwitchonE_Emotion E%20Emotion
    (:NewEnumerator0
      (Class|Image|SetBrushfromMaterial _image_emotion "/Game/DataTables/Dialogue/M_Neutral.M_Neutral"))
    (:NewEnumerator1
      (Class|Image|SetBrushfromMaterial _image_emotion "/Game/DataTables/Dialogue/M_Angry.M_Angry"))
    (:NewEnumerator2
      (Class|Image|SetBrushfromMaterial _image_emotion "/Game/DataTables/Dialogue/M_Excited.M_Excited"))
    (:NewEnumerator3
      (Class|Image|SetBrushfromMaterial _image_emotion "/Game/DataTables/Dialogue/M_Unamused.M_Unamused"))))

(event Custom|Set%20Speaker
  (params (E%20Speaker :type E_Speaker%20Enum :default "NewEnumerator0"))
  (bind _wb_dialogue_ref (Variables|Default|GetWB%20Dialogue%20Ref))
  (bind _image_speaker (Variables|/Game/DataTables/Dialogue/WB_Dialogue.WB_Dialogue_C|GetImage_Speaker _wb_dialogue_ref))
  (switch Utilities|FlowControl|Switch|SwitchonE_Speaker E%20Speaker
    (:NewEnumerator0
      (Class|Image|SetBrushfromMaterial _image_speaker "/Game/DataTables/Dialogue/M_Apple.M_Apple"))
    (:NewEnumerator1
      (Class|Image|SetBrushfromMaterial _image_speaker "/Game/DataTables/Dialogue/M_Orange.M_Orange"))
    (:NewEnumerator3
      (Class|Image|SetBrushfromMaterial _image_speaker "/Game/DataTables/Dialogue/M_Milk.M_Milk"))
    (:NewEnumerator4
      (Class|Image|SetBrushfromMaterial _image_speaker "/Game/DataTables/Dialogue/M_Egg.M_Egg"))))

(event Custom|Set%20Text
  (params (Text :type Text))
  (Variables|/Script/UMG.EditableText|SetText (Variables|/Game/DataTables/Dialogue/WB_Dialogue.WB_Dialogue_C|GetEditableText_0 (Variables|Default|GetWB%20Dialogue%20Ref)) Text))

(event Custom|Activate%20Dialogue
  (if (Variables|Default|GetDialogue)
    (Utilities|FlowControl|Sequence
      (:then_0
        (Utilities|FlowControl|DoOnce false
          (:Completed
            (UserInterface|Viewport|AddtoViewport (Variables|Default|GetWB%20Dialogue%20Ref) 0))))
      (:then_1
        (bind _outrownames (DataTable|GetDataTableRowNames "/Game/DataTables/Dialogue/DT_Dialogue.DT_Dialogue"))
        (if (< (Variables|Default|GetIndex) (Utilities|Array|Length _outrownames))
          (bind _returnvalue (Utilities|GetDataTableRow "/Game/DataTables/Dialogue/DT_Dialogue.DT_Dialogue" (Utilities|Array|Get(acopy) _outrownames (Variables|Default|GetIndex)))
            (:then
              (CallFunction|SetText (.text _returnvalue))
              (CallFunction|SetEmotion (.emotion _returnvalue))
              (CallFunction|SetSpeaker (.speaker _returnvalue))
              (Math|Integer|IncrementInt (Variables|Default|GetIndex))))
          (else
            (Variables|Default|SetIndex 0)
            (Variables|Default|SetDialogue false)
            (Widget|RemovefromParent (Variables|Default|GetWB%20Dialogue%20Ref))
            (CallFunction|ResetWidget)))))))

(event Custom|Reset%20Widget
  (Utilities|FlowControl|DoOnce false) ; enters at Reset
)

(event EventBeginPlay
  (bind _returnvalue (UserInterface|CreateWidget "/Game/DataTables/Dialogue/WB_Dialogue.WB_Dialogue_C" (Game|GetPlayerController 0)))
  (Variables|Default|SetWB%20Dialogue%20Ref _returnvalue)
  (bind _returnvalue_2 (UserInterface|CreateWidget "/Game/DataTables/Dialogue/WB_PressE.WB_PressE_C" (Game|GetPlayerController 0)))
  (Variables|Default|SetWB%20PressE%20Ref _returnvalue_2))

(fn ConstructionScript)